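; Item generator component that creates a randomized O_ItemData object from a random ItemTable row.
; CalculateRarity sets quality by weighted roll, then the item type decides the extras: Weapon and Utility get modifiers, Base and Head get utility and weapon slot configurations respectively.
; Modifiers are filtered by quality-based power cost limits and picked by weight, pruning duplicate types and those exceeding the remaining power budget.
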(fn GenerateItem
  (bind _itemtable (Variables|Default|GetItemTable))
  (Variables|Default|SetCachedItem 0)
  (bind _outrownames (DataTable|GetDataTableRowNames _itemtable))
  (bind _returnvalue (Utilities|GetDataTableRow _itemtable (Utilities|Array|Get(acopy) _outrownames (Math|Random|RandomIntegerinRange 0 (Utilities|Array|LastIndex _outrownames))))
    (:then
      (bind _returnvalue_2 (Game|ConstructObjectfromClass "/Game/Blueprint/O_ItemData.O_ItemData_C" (Components|GetOwner) _returnvalue))
      (Variables|Default|SetCachedItem _returnvalue_2)
      (Utilities|FlowControl|Sequence
        (:then_0
          (bind _quality (CallFunction|CalculateRarity 7.0 7.0 3.0 1.0))
          (|SetBy-RefVar (.Quality (Utilities|Struct|BreakBaseItemType (Variables|/Game/Blueprint/O_ItemData.O_ItemData_C|GetBaseType (Variables|Default|GetCachedItem)))) _quality))
        (:then_1
          (switch Utilities|FlowControl|Switch|SwitchonEItemType (.Type (Utilities|Struct|BreakBaseItemType (Variables|/Game/Blueprint/O_ItemData.O_ItemData_C|GetBaseType _returnvalue_2)))
            (:NewEnumerator0
              (CallFunction|SetRandomItemModifier "/Game/DataTables/WeaponModifiers.WeaponModifiers"))
            (:NewEnumerator1
              (CallFunction|SetRandomItemModifier "/Game/DataTables/UtilModifiers.UtilModifiers"))
            (:NewEnumerator2
              (CallFunction|ConfigUtilSlots))
            (:NewEnumerator3
              (CallFunction|ConfigWeaponSlots))))
        (:then_2
          (return (Variables|Default|GetCachedItem)))))))

(fn SetRandomItemModifier
  (params (ModifierTable :type Data%20Table%20Object%20Reference))
  (bind _cacheditem (Variables|Default|GetCachedItem))
  (bind _cacheditem_2 (Variables|Default|GetCachedItem))
  (bind _basetype (Variables|/Game/Blueprint/O_ItemData.O_ItemData_C|GetBaseType _cacheditem))
  (bind _modifiers (Variables|/Game/Blueprint/O_ItemData.O_ItemData_C|GetModifiers _cacheditem_2))
  (bind (_type _subtype _quality) (Utilities|Struct|BreakBaseItemType _basetype))
  (bind (_min _max) (CallFunction|GetModifierAmounts _quality))
  (LocalVariables|SetMinPowerLvlModifier (CallFunction|GetMinimalPowerCost _quality))
  (LocalVariables|SetMaxPower (CallFunction|GetPowerLevel _quality _type))
  (LocalVariables|SetModifierAmount (Math|Random|RandomIntegerinRange _min _max))
  (Utilities|FlowControl|Sequence
    (:then_0
      ;[1 1 1] Fill Table with aviable Mods
      (bind _outrownames (DataTable|GetDataTableRowNames ModifierTable))
      (for _array_element _outrownames
        (bind _returnvalue (Utilities|GetDataTableRow ModifierTable _array_element)
          (:then
            (if (and (>= (.PowerCost (Utilities|Struct|BreakValueModifierTable _returnvalue)) (LocalVariables|GetMinPowerLvlModifier)) (<= (.PowerCost (Utilities|Struct|BreakValueModifierTable _returnvalue)) (LocalVariables|GetMaxPower)))
              (Utilities|Array|Add (Variables|Default|GetAviableMods) _returnvalue)
              (LocalVariables|SetMaxWeighting (+ (.Weighting (Utilities|Struct|BreakValueModifierTable _returnvalue)) (LocalVariables|GetMaxWeighting))))))))
    (:then_1
      (LocalVariables|SetRandomValue (Math|Random|RandomFloatinRange 0.0 (LocalVariables|GetMaxWeighting)))
      ;[1 1 1] Roll Modifiers
      (while (and (> (Utilities|Array|Length (Variables|Default|GetAviableMods)) 0) (> (LocalVariables|GetModifierAmount) 0))
        (bind _array_element_2 (Utilities|Array|ForEachLoopwithBreak (Variables|Default|GetAviableMods) :!label _label)
          (:LoopBody
            (if (< (LocalVariables|GetRandomValue) (.Weighting (Utilities|Struct|BreakValueModifierTable _array_element_2)))
              (Math|Integer|DecrementInt (LocalVariables|GetModifierAmount)
                (:%20%20
                  (switch Utilities|FlowControl|Switch|SwitchonEModifierType (.Type (Utilities|Struct|BreakValueModifierTable _array_element_2))
                    (:NewEnumerator0
                      (Utilities|Array|Add _modifiers (Utilities|Struct|MakeFinalModifierValue (.Type (Utilities|Struct|BreakValueModifierTable _array_element_2)) (Math|Vector2D|MakeVector2D (Math|Random|RandomFloatinRange (.X (Math|Vector2D|BreakVector2D (.Range (Utilities|Struct|BreakValueModifierTable _array_element_2)))) (.Y (Math|Vector2D|BreakVector2D (.Range (Utilities|Struct|BreakValueModifierTable _array_element_2))))) 0.0)) :!label _label_2) ; Single Value
                    )
                    (:NewEnumerator1
                      (goto _label_2))
                    (:NewEnumerator3
                      (Utilities|Array|Add _modifiers (Utilities|Struct|MakeFinalModifierValue (.Type (Utilities|Struct|BreakValueModifierTable _array_element_2)) (.Range (Utilities|Struct|BreakValueModifierTable _array_element_2)))) ; Range Value
                    )
                    (:NewEnumerator2
                      (goto _label_2))
                    (:NewEnumerator4
                      (goto _label_2)))
                  (LocalVariables|SetMaxPower (- (LocalVariables|GetMaxPower) (.PowerCost (Utilities|Struct|BreakValueModifierTable _array_element_2))))
                  (goto _label Break)))
              (else
                (LocalVariables|SetRandomValue (- (LocalVariables|GetRandomValue) (.Weighting (Utilities|Struct|BreakValueModifierTable _array_element_2)))))))
          (:Completed
            ;[1 1 1] Remove same Modifier Type from aviable Mods
            (bind _arrayelement (Utilities|Array|ReverseforEachLoop (Variables|Default|GetAviableMods))
              (:LoopBody
                (for _array_element_3 (Variables|/Game/Blueprint/O_ItemData.O_ItemData_C|GetModifiers (Variables|Default|GetCachedItem))
                  (if (or (== (.Type (Utilities|Struct|BreakFinalModifierValue _array_element_3)) (.Type (Utilities|Struct|BreakValueModifierTable _arrayelement))) (> (.PowerCost (Utilities|Struct|BreakValueModifierTable _arrayelement)) (LocalVariables|GetMaxPower)))
                    (Utilities|Array|RemoveItem (Variables|Default|GetAviableMods) _arrayelement)))))))))))

(fn ConfigWeaponSlots
  (Variables|/Game/Blueprint/O_ItemData.O_ItemData_C|SetSlotModifier (Variables|Default|GetCachedItem) (Utilities|Select :Index (Math|Random|RandomIntegerinRange 0 2) :Option%200 (Utilities|Struct|MakeSlotModifier "NewEnumerator1" (Math|Random|RandomIntegerinRange 2 4)) :Option%201 (Utilities|Struct|MakeSlotModifier "NewEnumerator2" (Math|Random|RandomIntegerinRange 1 2)) :Option%202 (Utilities|Struct|MakeSlotModifier "NewEnumerator3" 1))))

(fn ConfigUtilSlots
  (Variables|/Game/Blueprint/O_ItemData.O_ItemData_C|SetSlotModifier (Variables|Default|GetCachedItem) (Utilities|Select :Index (Math|Random|RandomIntegerinRange 0 2) :Option%200 (Utilities|Struct|MakeSlotModifier "NewEnumerator0" (Math|Random|RandomIntegerinRange 0 1)) :Option%201 (Utilities|Struct|MakeSlotModifier "NewEnumerator0" (Math|Random|RandomIntegerinRange 0 2)) :Option%202 (Utilities|Struct|MakeSlotModifier "NewEnumerator0" (Math|Random|RandomIntegerinRange 1 2)))))

(fn CalculateRarity
  (params (Common :type Float%20%28single-precision%29) (Uncommon :type Float%20%28single-precision%29) (Rare :type Float%20%28single-precision%29) (Epic :type Float%20%28single-precision%29))
  (bind _array (Utilities|Array|MakeArray Common Uncommon Rare Epic))
  (for _array_element _array
    (LocalVariables|SetWeighingSum (+ _array_element (LocalVariables|GetWeighingSum))))
  (LocalVariables|SetRandom%20Value (Math|Random|RandomFloatinRange 0.0 (LocalVariables|GetWeighingSum)))
  (for (_array_element_2 _array_index) _array
    (if (< (LocalVariables|GetRandom%20Value) _array_element_2)
      (return (Utilities|Enum|ByteToEnumEQuality (Math|Conversions|ToByte(Integer) _array_index)))
      (else
        (LocalVariables|SetRandom%20Value (- (LocalVariables|GetRandom%20Value) _array_element_2))))))