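; Blueprint function library of helpers for the item-based tower system, mapping item quality and type to balance values and computing final tower stats.
; Quality lookups return the display color, modifier count range, minimum power cost, and a power level that also varies by item type.
; CalculateTowerValues takes base stats from the Weapon item and sums all item and tower modifiers.
; Absolute bonuses apply before percentage bonuses for damage, speed, range and tracking.
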(fn GetQualityColor
  (params (Quality :type EQuality%20Enum :default "NewEnumerator0"))
  (return (Utilities|Select :Index Quality :NewEnumerator0 "(R=1.000000,G=1.000000,B=1.000000,A=1.000000)" :NewEnumerator1 "(R=0.117647,G=1.000000,B=0.000000,A=1.000000)" :NewEnumerator2 "(R=0.000000,G=0.439216,B=0.866667,A=1.000000)" :NewEnumerator3 "(R=0.639216,G=0.207843,B=0.933333,A=1.000000)")))

(fn GetPowerLevel
  (params (Quality :type EQuality%20Enum :default "NewEnumerator0") (Type :type EItemType%20Enum :default "NewEnumerator0"))
  (switch Utilities|FlowControl|Switch|SwitchonEItemType Type
    (:NewEnumerator0
      ;[1 1 1] Weapon
      (return (Utilities|Select :Index Quality :NewEnumerator0 8 :NewEnumerator1 20 :NewEnumerator2 40 :NewEnumerator3 80)))
    (:NewEnumerator1
      ;[1 1 1] Utility
      (return (Utilities|Select :Index Quality :NewEnumerator0 8 :NewEnumerator1 20 :NewEnumerator2 35 :NewEnumerator3 60)))
    (:NewEnumerator2
      ;[1 1 1] Base
      (return (Utilities|Select :Index Quality :NewEnumerator0 10 :NewEnumerator1 20 :NewEnumerator2 35 :NewEnumerator3 50)))
    (:NewEnumerator3
      ;[1 1 1] Head
      (return (Utilities|Select :Index Quality :NewEnumerator0 10 :NewEnumerator1 20 :NewEnumerator2 35 :NewEnumerator3 50)))
    (:NewEnumerator4
      ;[1 1 1] Ammo
      (return (Utilities|Select :Index Quality :NewEnumerator0 10 :NewEnumerator1 20 :NewEnumerator2 35 :NewEnumerator3 50)))))

(fn GetModifierAmounts
  (params (Quality :type EQuality%20Enum :default "NewEnumerator0"))
  (switch Utilities|FlowControl|Switch|SwitchonEQuality Quality
    (:NewEnumerator0
      (return 0 1))
    (:NewEnumerator1
      (return 1 2))
    (:NewEnumerator2
      (return 1 3))
    (:NewEnumerator3
      (return 2 4))))

(fn GetMinimalPowerCost
  (params (Quality :type EQuality%20Enum :default "NewEnumerator0"))
  (return (Utilities|Select :Index Quality :NewEnumerator0 0 :NewEnumerator1 5 :NewEnumerator2 10 :NewEnumerator3 20)))

(fn CalculateTowerValues
  (params (TowerItems :type Array%20of%20O%20Item%20Data%20Object%20References) (TowerModifier :type Array%20of%20Final%20Modifier%20Value%20Structures))
  (for _array_element TowerItems
    (if (Utilities|Enum|Equal(Enum) (.Type (Utilities|Struct|BreakBaseItemType (Variables|/Game/Blueprint/O_ItemData.O_ItemData_C|GetBaseType _array_element))) "NewEnumerator0")
      (LocalVariables|SetBaseValue (.BaseValues (Utilities|Struct|BreakBaseItemType (Variables|/Game/Blueprint/O_ItemData.O_ItemData_C|GetBaseType _array_element)))))
    ;[1 1 1] Item Modifiers
    (for _array_element_2 (Variables|/Game/Blueprint/O_ItemData.O_ItemData_C|GetModifiers _array_element)
      (switch Utilities|FlowControl|Switch|SwitchonEModifierType (.Type (Utilities|Struct|BreakFinalModifierValue _array_element_2))
        (:NewEnumerator1
          (LocalVariables|SetP_DMG (+ (LocalVariables|GetP_DMG) (.X (Math|Vector2D|BreakVector2D (.Value (Utilities|Struct|BreakFinalModifierValue _array_element_2)))))))
        (:NewEnumerator3
          (LocalVariables|SetA_DMG (+ (LocalVariables|GetA_DMG) (.Value (Utilities|Struct|BreakFinalModifierValue _array_element_2)))))
        (:NewEnumerator5
          (LocalVariables|SetP_Range (+ (LocalVariables|GetP_Range) (.X (Math|Vector2D|BreakVector2D (.Value (Utilities|Struct|BreakFinalModifierValue _array_element_2)))))))
        (:NewEnumerator2
          (LocalVariables|SetA_Range (+ (LocalVariables|GetA_Range) (.X (Math|Vector2D|BreakVector2D (.Value (Utilities|Struct|BreakFinalModifierValue _array_element_2)))))))
        (:NewEnumerator4
          (LocalVariables|SetP_Tracking (+ (LocalVariables|GetP_Tracking) (.X (Math|Vector2D|BreakVector2D (.Value (Utilities|Struct|BreakFinalModifierValue _array_element_2)))))))
        (:NewEnumerator6
          (LocalVariables|SetA_Tracking (+ (LocalVariables|GetA_Tracking) (.X (Math|Vector2D|BreakVector2D (.Value (Utilities|Struct|BreakFinalModifierValue _array_element_2)))))))
        (:NewEnumerator7
          (LocalVariables|SetP_Speed (+ (LocalVariables|GetP_Speed) (.X (Math|Vector2D|BreakVector2D (.Value (Utilities|Struct|BreakFinalModifierValue _array_element_2)))))))
        (:NewEnumerator8
          (LocalVariables|SetA_Speed (+ (LocalVariables|GetA_Speed) (.X (Math|Vector2D|BreakVector2D (.Value (Utilities|Struct|BreakFinalModifierValue _array_element_2))))))))))
  ;[1 1 1] Tower Modifiers
  (for _array_element_3 TowerModifier
    (switch Utilities|FlowControl|Switch|SwitchonEModifierType (.Type (Utilities|Struct|BreakFinalModifierValue _array_element_3))
      (:NewEnumerator1
        (LocalVariables|SetP_DMG (+ (LocalVariables|GetP_DMG) (.X (Math|Vector2D|BreakVector2D (.Value (Utilities|Struct|BreakFinalModifierValue _array_element_3)))))))
      (:NewEnumerator3
        (LocalVariables|SetA_DMG (+ (LocalVariables|GetA_DMG) (.Value (Utilities|Struct|BreakFinalModifierValue _array_element_3)))))
      (:NewEnumerator5
        (LocalVariables|SetP_Range (+ (LocalVariables|GetP_Range) (.X (Math|Vector2D|BreakVector2D (.Value (Utilities|Struct|BreakFinalModifierValue _array_element_3)))))))
      (:NewEnumerator2
        (LocalVariables|SetA_Range (+ (LocalVariables|GetA_Range) (.X (Math|Vector2D|BreakVector2D (.Value (Utilities|Struct|BreakFinalModifierValue _array_element_3)))))))
      (:NewEnumerator4
        (LocalVariables|SetP_Tracking (+ (LocalVariables|GetP_Tracking) (.X (Math|Vector2D|BreakVector2D (.Value (Utilities|Struct|BreakFinalModifierValue _array_element_3)))))))
      (:NewEnumerator6
        (LocalVariables|SetA_Tracking (+ (LocalVariables|GetA_Tracking) (.X (Math|Vector2D|BreakVector2D (.Value (Utilities|Struct|BreakFinalModifierValue _array_element_3)))))))
      (:NewEnumerator7
        (LocalVariables|SetP_Speed (+ (LocalVariables|GetP_Speed) (.X (Math|Vector2D|BreakVector2D (.Value (Utilities|Struct|BreakFinalModifierValue _array_element_3)))))))
      (:NewEnumerator8
        (LocalVariables|SetA_Speed (+ (LocalVariables|GetA_Speed) (.X (Math|Vector2D|BreakVector2D (.Value (Utilities|Struct|BreakFinalModifierValue _array_element_3)))))))))
  (return (Utilities|Struct|MakeBaseItemValues (+ (+ (.Damage (Utilities|Struct|BreakBaseItemValues (LocalVariables|GetBaseValue))) (LocalVariables|GetA_DMG)) (* (+ (.Damage (Utilities|Struct|BreakBaseItemValues (LocalVariables|GetBaseValue))) (LocalVariables|GetA_DMG)) (* (LocalVariables|GetP_DMG) 0.01))) (+ (+ (.Speed (Utilities|Struct|BreakBaseItemValues (LocalVariables|GetBaseValue))) (LocalVariables|GetA_Speed)) (* (+ (.Speed (Utilities|Struct|BreakBaseItemValues (LocalVariables|GetBaseValue))) (LocalVariables|GetA_Speed)) (* (LocalVariables|GetP_Speed) 0.01))) (+ (+ (.Range (Utilities|Struct|BreakBaseItemValues (LocalVariables|GetBaseValue))) (LocalVariables|GetA_Range)) (* (+ (.Range (Utilities|Struct|BreakBaseItemValues (LocalVariables|GetBaseValue))) (LocalVariables|GetA_Range)) (* (LocalVariables|GetP_Range) 0.01))) (+ (+ (.Trackingspeed (Utilities|Struct|BreakBaseItemValues (LocalVariables|GetBaseValue))) (LocalVariables|GetA_Tracking)) (* (+ (.Trackingspeed (Utilities|Struct|BreakBaseItemValues (LocalVariables|GetBaseValue))) (LocalVariables|GetA_Tracking)) (* (LocalVariables|GetP_Tracking) 0.01))))))