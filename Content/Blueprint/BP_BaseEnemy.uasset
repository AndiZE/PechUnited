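; BP_BaseEnemy is a base enemy pawn that takes projectile damage and is destroyed when its health runs out.
; On BeginPlay it writes the first waypoint of its Path into its controller's Blackboard under the Waypoint key.
; The construction script initializes current health from MaxHealth and applies Speed to the FloatingPawnMovement component's max speed.
; OnProjectileHit subtracts damage from health and destroys the actor at zero or below.
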(event Custom|OnProjectileHit
  (params (Damage :type Integer))
  (bind _output_get (Variables|BaseStats|SetCurrentHealth (- (Variables|BaseStats|GetCurrentHealth) Damage)))
  (if (<= _output_get 0)
    (Actor|DestroyActor)))

(event EventBeginPlay
  (AI|Components|Blackboard|SetValueasObject (AI|GetBlackboard (Pawn|GetController)) (Utilities|Name|MakeLiteralName "Waypoint") (Utilities|Array|Get(acopy) (Variables|/Game/Blueprint/BP_Path.BP_Path_C|GetWaypoints (Variables|Default|GetPath)))))

(fn ConstructionScript
  (Variables|BaseStats|SetCurrentHealth (Variables|BaseStats|GetMaxHealth))
  (Variables|/Script/Engine.FloatingPawnMovement|SetMaxSpeed (Variables|Default|GetFloatingPawnMovement) (Variables|BaseStats|GetSpeed)))