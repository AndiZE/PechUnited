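; BP_BaseProjectile is a base homing projectile that flies at a target actor and deals damage on arrival.
; Each Tick it moves at Speed toward a point slightly above the target's origin and rotates to face it.
; A distance check replaces collision: within a small radius it passes Damage to the target's OnProjectileHit and destroys itself.
; It also destroys itself if the target becomes invalid.
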(event EventTick
  (params (DeltaSeconds :type Float%20%28single-precision%29))
  (bind _returnvalue (Transformation|GetActorLocation))
  (bind _target (Variables|Default|GetTarget))
  (bind _returnvalue_2 (Transformation|GetActorLocation _target))
  (bind _returnvalue_3 (+ _returnvalue_2 "0, 0,80.000000"))
  (bind _returnvalue_4 (- _returnvalue_3 _returnvalue))
  (Utilities|IsValid (Variables|Default|GetTarget)
    (:Is%20Valid
      (Transformation|SetActorLocationAndRotation (+ _returnvalue (* (Math|Vector|Normalize _returnvalue_4) (* (Variables|Default|GetSpeed) (Utilities|Time|GetWorldDeltaSeconds)))) (Math|Rotator|MakeRotfromX _returnvalue_4))
      (if (<= (Math|Vector|Distance(Vector) (+ (Transformation|GetActorLocation (Variables|Default|GetTarget)) "0, 0,80.000000") (Transformation|GetActorLocation)) 2e+01)
        (Default|OnProjectileHit (Variables|Default|GetTarget) (Variables|Default|GetDamage))
        (Actor|DestroyActor)))
    (:Is%20Not%20Valid
      (Actor|DestroyActor))))

(fn ConstructionScript)