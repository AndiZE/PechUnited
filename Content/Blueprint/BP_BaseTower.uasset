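; Base tower Blueprint that automatically fires projectiles at enemies within its range.
; A sphere sized from Range in the construction script tracks overlapping enemies, accepting air units only if CanAttackAir is set.
; It holds one target until that target leaves the sphere, then takes the first remaining in the list.
; A Tick timer fires at Speed shots per second, spawning a projectile with the target and random damage.
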(event OnComponentBeginOverlap(Sphere)
  (params (OverlappedComponent :type Primitive%20Component%20Object%20Reference) (OtherActor :type Actor%20Object%20Reference) (OtherComp :type Primitive%20Component%20Object%20Reference) (OtherBodyIndex :type Integer) (bFromSweep :type Boolean) (SweepResult :type Hit%20Result%20Structure%20%28by%20ref%29))
  ;[1 1 1] Add Enemy Targets to List
  (bind _asbp_base_enemy (Utilities|Casting|CastToBP_BaseEnemy OtherActor))
  (if (Variables|/Game/Blueprint/BP_BaseEnemy.BP_BaseEnemy_C|GetIsAir _asbp_base_enemy)
    (if (Variables|MainStats|GetCanAttackAir)
      (Utilities|Array|AddUnique (Variables|Default|GetAviableTargets) _asbp_base_enemy :!label _label)
      ;[1 1 1] If no Current Target is Set, use current entered Enemy
      (Utilities|IsValid (Variables|Default|GetCurrentTarget)
        (:Is%20Not%20Valid
          (Variables|Default|SetCurrentTarget _asbp_base_enemy))))
    (else
      (goto _label))))

(event OnComponentEndOverlap(Sphere)
  (params (OverlappedComponent :type Primitive%20Component%20Object%20Reference) (OtherActor :type Actor%20Object%20Reference) (OtherComp :type Primitive%20Component%20Object%20Reference) (OtherBodyIndex :type Integer))
  ;[1 1 1] Remove Enemy Targets to List
  (bind _asbp_base_enemy (Utilities|Casting|CastToBP_BaseEnemy OtherActor))
  (if (Utilities|Array|ContainsItem (Variables|Default|GetAviableTargets) _asbp_base_enemy)
    (Utilities|Array|RemoveItem (Variables|Default|GetAviableTargets) _asbp_base_enemy))
  ;[1 1 1] Check if current target left Towerrange, get Next from List
  (if (== _asbp_base_enemy (Variables|Default|GetCurrentTarget))
    (CallFunction|SetNextTarget)))

(event EventTick
  (params (DeltaSeconds :type Float%20%28single-precision%29))
  ;[1 1 1] Update Internal Timer every Frame
  (Variables|Default|SetShootTimer (+ (Utilities|Time|GetWorldDeltaSeconds) (Variables|Default|GetShootTimer)))
  ;[1 1 1] Check if Any Targets Aviable and if Enough Time Pass to Fire one Shot
  (if (and (>= (Variables|Default|GetShootTimer) (/ (/ 6e+01 (Variables|MainStats|GetSpeed)) 6e+01)) (Utilities|IsValid (Variables|Default|GetCurrentTarget)))
    (CallFunction|Shoot)
    (Variables|Default|SetShootTimer 0.0) ; Reset Timer
  ))

(fn ConstructionScript
  (Components|Sphere|SetSphereRadius (Variables|Default|GetSphere) (Variables|MainStats|GetRange) true))

(fn Shoot
  (bind _projectilespawnpoint (Variables|Default|GetProjectileSpawnPoint))
  (bind _returnvalue (Transformation|GetWorldLocation _projectilespawnpoint))
  (Game|SpawnActorfromClass "/Game/Blueprint/BP_BaseProjectile.BP_BaseProjectile_C" (Math|Transform|MakeTransform _returnvalue (Math|Rotator|MakeRotfromX (- (Transformation|GetActorLocation (Variables|Default|GetCurrentTarget)) _returnvalue)) "1,1,1") "AlwaysSpawn" 0 (Math|Random|RandomIntegerinRange (Variables|MainStats|GetMinDamage) (Variables|MainStats|GetMaxDamage)) (Variables|Default|GetCurrentTarget) 0))

(fn SetNextTarget
  ;[1 1 1] Are Targets aviable in List?
  (if (> (Utilities|Array|Length (Variables|Default|GetAviableTargets)) 0)
    (Variables|Default|SetCurrentTarget (Utilities|Array|Get(acopy) (Variables|Default|GetAviableTargets))) ; Get Next Target from List
    (else
      (Variables|Default|SetCurrentTarget 0) ; No Target aviable
    )))