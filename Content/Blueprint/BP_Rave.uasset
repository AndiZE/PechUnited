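; BP_Rave is an actor whose static mesh flashes random colors every frame, like a rave light.
; On BeginPlay it creates a dynamic material instance from the mesh's first material slot and stores it.
; Each Tick it sets that instance's Color vector parameter to a new random, fully opaque RGB value, with no timing or smoothing between changes.
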(event EventTick
  (params (DeltaSeconds :type Float%20%28single-precision%29))
  (Rendering|Material|SetVectorParameterValue (Variables|Default|GetMaterial) "Color" (Utilities|Struct|MakeLinearColor (Math|Random|RandomFloatinRange 0.0 1.0) (Math|Random|RandomFloatinRange 0.0 1.0) (Math|Random|RandomFloatinRange 0.0 1.0) 1.0) :!class /Script/Engine.MaterialInstanceDynamic))

(event EventBeginPlay
  (bind _staticmesh (Variables|Default|GetStaticMesh))
  (bind _returnvalue (Rendering|Material|CreateDynamicMaterialInstance _staticmesh 0 (Rendering|Material|GetMaterial _staticmesh 0) "None" :!class /Script/Engine.PrimitiveComponent))
  (Variables|Default|SetMaterial _returnvalue))

(fn ConstructionScript)