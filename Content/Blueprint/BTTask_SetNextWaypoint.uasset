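; Behavior tree task that advances a BP_BaseEnemy to the next waypoint on its path.
; It reads the current waypoint from the blackboard, asks the enemy's Path for the following one, and writes a valid result back to the same key.
; The task finishes successfully only in that case; an invalid result has no FinishExecute call.
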(event EventReceiveExecuteAI
  (params (OwnerController :type AI%20Controller%20Object%20Reference) (ControlledPawn :type Pawn%20Object%20Reference))
  (bind _next (Default|GetNextWaypoint (Variables|/Game/Blueprint/BP_BaseEnemy.BP_BaseEnemy_C|GetPath (.AsBP%20Base%20Enemy (Utilities|Casting|CastToBP_BaseEnemy ControlledPawn))) (.AsBP%20Waypoint (Utilities|Casting|CastToBP_Waypoint (Class|BTFunctionLibrary|GetBlackboardValueasObject (Variables|Default|GetWaypoint))))))
  (Utilities|IsValid _next
    (:Is%20Valid
      (Class|BTFunctionLibrary|SetBlackboardValueasObject (Variables|Default|GetWaypoint) _next)
      (AI|BehaviorTree|FinishExecute true))))