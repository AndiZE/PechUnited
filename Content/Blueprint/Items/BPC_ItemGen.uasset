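; Item generator component that builds a randomized item data object from a random row of the item table.
; It rolls quality by weighted chance, then branches by item type to choose allowed modifiers and a modifier table, adding slot configurations for Head and Base items.
; Modifiers are filtered by a type bitmask and cost, then picked by weight within a quality-based count and power budget, pruning duplicate types.
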(fn GenerateItem
  (bind _itemtable (Variables|Default|GetItemTable))
  (Variables|Default|SetCachedItem 0)
  (bind _outrownames (DataTable|GetDataTableRowNames _itemtable))
  (bind _returnvalue (Utilities|GetDataTableRow _itemtable (Utilities|Array|Get(acopy) _outrownames (Math|Random|RandomIntegerinRange 0 (Utilities|Array|LastIndex _outrownames))))
    (:then
      (bind _returnvalue_2 (Game|ConstructObjectfromClass "/Game/Blueprint/Items/O_ItemData.O_ItemData_C" (Components|GetOwner) _returnvalue))
      (Variables|Default|SetCachedItem _returnvalue_2)
      (Utilities|FlowControl|Sequence
        (:then_0
          (bind _quality (CallFunction|CalculateRarity 7.0 7.0 3.0 1.0))
          (|SetBy-RefVar (.Quality (Utilities|Struct|BreakBaseItemType (Variables|/Game/Blueprint/Items/O_ItemData.O_ItemData_C|GetBaseType (Variables|Default|GetCachedItem)))) _quality))
        (:then_1
          (switch Utilities|FlowControl|Switch|SwitchonEItemType (.Type (Utilities|Struct|BreakBaseItemType (Variables|/Game/Blueprint/Items/O_ItemData.O_ItemData_C|GetBaseType _returnvalue_2)))
            (:NewEnumerator0
              (CallFunction|GenerateWeapon (.Size (Utilities|Struct|BreakBaseItemType (Variables|/Game/Blueprint/Items/O_ItemData.O_ItemData_C|GetBaseType _returnvalue_2)))))
            (:NewEnumerator1
              (CallFunction|GenerateUtility))
            (:NewEnumerator2
              (CallFunction|GenerateBase))
            (:NewEnumerator3
              (CallFunction|GenerateHead))
            (:NewEnumerator4
              (CallFunction|GenerateAmmo))))
        (:then_2
          (return (Variables|Default|GetCachedItem)))))))

(fn SetRandomItemModifier
  (params (ModifierTable :type Data%20Table%20Object%20Reference))
  (bind _cacheditem (Variables|Default|GetCachedItem))
  (bind _cacheditem_2 (Variables|Default|GetCachedItem))
  (bind _basetype (Variables|/Game/Blueprint/Items/O_ItemData.O_ItemData_C|GetBaseType _cacheditem))
  (bind _modifiers (Variables|/Game/Blueprint/Items/O_ItemData.O_ItemData_C|GetModifiers _cacheditem_2))
  (bind (_type _subtype _quality) (Utilities|Struct|BreakBaseItemType _basetype))
  (bind (_min _max) (CallFunction|GetModifierAmounts _quality))
  (LocalVariables|SetMinPowerLvlModifier (CallFunction|GetMinimalPowerCost _quality))
  (LocalVariables|SetMaxPower (CallFunction|GetPowerLevel _quality _type))
  (LocalVariables|SetModifierAmount (Math|Random|RandomIntegerinRange _min _max))
  (Utilities|FlowControl|Sequence
    (:then_0
      ;[1 1 1] Fill Table with aviable Mods
      (bind _outrownames (DataTable|GetDataTableRowNames ModifierTable))
      (for _array_element _outrownames
        (bind _returnvalue (Utilities|GetDataTableRow ModifierTable _array_element)
          (:then
            (bind _allowed (CallFunction|ModifierAllowed (.Type (Utilities|Struct|BreakTableModifierValues _returnvalue))))
            (if _allowed
              (if (and (>= (.Cost (Utilities|Struct|BreakTableModifierValues _returnvalue)) (LocalVariables|GetMinPowerLvlModifier)) (<= (.Cost (Utilities|Struct|BreakTableModifierValues _returnvalue)) (LocalVariables|GetMaxPower)))
                (Utilities|Array|Add (LocalVariables|GetAviableMods) _returnvalue)
                (LocalVariables|SetMaxWeighting (+ (.Weighting (Utilities|Struct|BreakTableModifierValues _returnvalue)) (LocalVariables|GetMaxWeighting)))))))))
    (:then_1
      (LocalVariables|SetRandomValue (Math|Random|RandomFloatinRange 0.0 (LocalVariables|GetMaxWeighting)))
      ;[1 1 1] Roll Modifiers
      (while (and (> (Utilities|Array|Length (LocalVariables|GetAviableMods)) 0) (> (LocalVariables|GetModifierAmount) 0))
        (bind _array_element_2 (Utilities|Array|ForEachLoopwithBreak (LocalVariables|GetAviableMods) :!label _label)
          (:LoopBody
            (if (< (LocalVariables|GetRandomValue) (.Weighting (Utilities|Struct|BreakTableModifierValues _array_element_2)))
              (Math|Integer|DecrementInt (LocalVariables|GetModifierAmount)
                (:%20%20
                  (switch Utilities|FlowControl|Switch|SwitchonEModifierType (.Type (Utilities|Struct|BreakTableModifierValues _array_element_2))
                    (:NewEnumerator1
                      (Utilities|Array|Add _modifiers (Utilities|Struct|MakeFinalModifierValue (.Type (Utilities|Struct|BreakTableModifierValues _array_element_2)) (Math|Vector2D|MakeVector2D (Math|Random|RandomFloatinRange (.X (Math|Vector2D|BreakVector2D (.Range (Utilities|Struct|BreakTableModifierValues _array_element_2)))) (.Y (Math|Vector2D|BreakVector2D (.Range (Utilities|Struct|BreakTableModifierValues _array_element_2))))) 0.0)) :!label _label_2) ; Single Value
                    )
                    (:NewEnumerator3
                      (Utilities|Array|Add _modifiers (Utilities|Struct|MakeFinalModifierValue (.Type (Utilities|Struct|BreakTableModifierValues _array_element_2)) (.Range (Utilities|Struct|BreakTableModifierValues _array_element_2)))) ; Range Value
                    )
                    (:NewEnumerator5
                      (goto _label_2))
                    (:NewEnumerator2
                      (goto _label_2))
                    (:NewEnumerator4
                      (goto _label_2))
                    (:NewEnumerator6
                      (goto _label_2))
                    (:NewEnumerator7
                      (goto _label_2))
                    (:NewEnumerator8
                      (goto _label_2)))
                  (LocalVariables|SetMaxPower (- (LocalVariables|GetMaxPower) (.Cost (Utilities|Struct|BreakTableModifierValues _array_element_2))))
                  (goto _label Break)))
              (else
                (LocalVariables|SetRandomValue (- (LocalVariables|GetRandomValue) (.Weighting (Utilities|Struct|BreakTableModifierValues _array_element_2)))))))
          (:Completed
            ;[1 1 1] Remove same Modifier Type from aviable Mods
            (bind (_arrayindex _arrayelement) (Utilities|Array|ReverseforEachLoop (LocalVariables|GetAviableMods))
              (:LoopBody
                (bind _array_element_3 (Utilities|Array|ForEachLoopwithBreak (Variables|/Game/Blueprint/Items/O_ItemData.O_ItemData_C|GetModifiers (Variables|Default|GetCachedItem)) :!label _label_3)
                  (:LoopBody
                    (if (or (== (.Type (Utilities|Struct|BreakFinalModifierValue _array_element_3)) (.Type (Utilities|Struct|BreakTableModifierValues _arrayelement))) (> (.Cost (Utilities|Struct|BreakTableModifierValues _arrayelement)) (LocalVariables|GetMaxPower)))
                      (Utilities|Array|RemoveIndex (LocalVariables|GetAviableMods) _arrayindex)
                      (goto _label_3 Break))))))))))))

(fn ConfigWeaponSlots
  (Variables|/Game/Blueprint/Items/O_ItemData.O_ItemData_C|SetSlotModifier (Variables|Default|GetCachedItem) (Utilities|Select :Index (Math|Random|RandomIntegerinRange 0 2) :Option%200 (Utilities|Struct|MakeSlotModifier "NewEnumerator1" (Math|Random|RandomIntegerinRange 2 4)) :Option%201 (Utilities|Struct|MakeSlotModifier "NewEnumerator2" (Math|Random|RandomIntegerinRange 1 2)) :Option%202 (Utilities|Struct|MakeSlotModifier "NewEnumerator3" 1))))

(fn ConfigUtilSlots
  (Variables|/Game/Blueprint/Items/O_ItemData.O_ItemData_C|SetSlotModifier (Variables|Default|GetCachedItem) (Utilities|Select :Index (Math|Random|RandomIntegerinRange 0 2) :Option%200 (Utilities|Struct|MakeSlotModifier "NewEnumerator0" (Math|Random|RandomIntegerinRange 0 1)) :Option%201 (Utilities|Struct|MakeSlotModifier "NewEnumerator0" (Math|Random|RandomIntegerinRange 0 2)) :Option%202 (Utilities|Struct|MakeSlotModifier "NewEnumerator0" (Math|Random|RandomIntegerinRange 1 2)))))

(fn CalculateRarity
  (params (Common :type Float%20%28single-precision%29) (Uncommon :type Float%20%28single-precision%29) (Rare :type Float%20%28single-precision%29) (Epic :type Float%20%28single-precision%29))
  (bind _array (Utilities|Array|MakeArray Common Uncommon Rare Epic))
  (for _array_element _array
    (LocalVariables|SetWeighingSum (+ _array_element (LocalVariables|GetWeighingSum))))
  (LocalVariables|SetRandom%20Value (Math|Random|RandomFloatinRange 0.0 (LocalVariables|GetWeighingSum)))
  (for (_array_element_2 _array_index) _array
    (if (< (LocalVariables|GetRandom%20Value) _array_element_2)
      (return (Utilities|Enum|ByteToEnumEQuality (Math|Conversions|ToByte(Integer) _array_index)))
      (else
        (LocalVariables|SetRandom%20Value (- (LocalVariables|GetRandom%20Value) _array_element_2))))))

(fn ConfigModifierFlag
  (params (ModifierCategory :type Array%20of%20EModifierType%20Enums :default "NewEnumerator1"))
  (Variables|Default|SetModifierFlag 0)
  (for _array_element ModifierCategory
    (Variables|Default|SetModifierFlag (Class|KismetMathLibrary|OrIntInt (Math|Float|Floor (Math|Float|Power 2.0 (Math|Conversions|ToFloat(Byte) _array_element))) (Variables|Default|GetModifierFlag)))))

(fn ModifierAllowed
  (params (Type :type EModifierType%20Enum :default "NewEnumerator1"))
  (return (Math|Conversions|ToBoolean(Integer) (Class|KismetMathLibrary|AndIntInt (Variables|Default|GetModifierFlag) (Math|Float|Floor (Math|Float|Power 2.0 (Math|Conversions|ToFloat(Byte) Type)))))))

(fn GenerateWeapon
  (params (Size :type EItemSize%20Enum :default "NewEnumerator0"))
  (CallFunction|ConfigModifierFlag (Utilities|Array|MakeArray "NewEnumerator1" "NewEnumerator3" "NewEnumerator5" "NewEnumerator2" "NewEnumerator4" "NewEnumerator6" "NewEnumerator7" "NewEnumerator8"))
  (CallFunction|SetRandomItemModifier (Utilities|Select :Index Size :NewEnumerator0 0 :NewEnumerator1 "/Game/DataTables/ItemTables/WeaponSmall.WeaponSmall" :NewEnumerator2 "/Game/DataTables/ItemTables/WeaponMedium.WeaponMedium" :NewEnumerator3 "/Game/DataTables/ItemTables/WeaponLarge.WeaponLarge")))

(fn GenerateHead
  (CallFunction|ConfigModifierFlag (Utilities|Array|MakeArray "NewEnumerator5" "NewEnumerator7" "NewEnumerator4"))
  (CallFunction|SetRandomItemModifier "/Game/DataTables/Modifiers/Percent_General.Percent_General")
  (CallFunction|ConfigWeaponSlots))

(fn GenerateBase
  (CallFunction|ConfigModifierFlag (Utilities|Array|MakeArray "NewEnumerator5" "NewEnumerator4"))
  (CallFunction|SetRandomItemModifier "/Game/DataTables/Modifiers/Percent_General.Percent_General")
  (CallFunction|ConfigUtilSlots))

(fn GenerateUtility
  (CallFunction|ConfigModifierFlag (Utilities|Array|MakeArray "NewEnumerator5" "NewEnumerator4" "NewEnumerator1" "NewEnumerator7"))
  (CallFunction|SetRandomItemModifier "/Game/DataTables/Modifiers/Percent_General.Percent_General"))

(fn GenerateAmmo
  (CallFunction|ConfigModifierFlag (Utilities|Array|MakeArray "NewEnumerator5" "NewEnumerator1" "NewEnumerator7"))
  (CallFunction|SetRandomItemModifier "/Game/DataTables/Modifiers/Percent_General.Percent_General"))