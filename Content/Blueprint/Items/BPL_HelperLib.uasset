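; Blueprint function library of item helpers that map quality tiers, from Common to Epic, to item properties.
; Independent hardcoded lookups supply each tier's display color, modifier count range and minimal power cost.
; Power level also depends on item type: Weapon and Utility scale with quality, while Base, Head and Ammo always return zero.
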(fn GetQualityColor
  (params (Quality :type EQuality%20Enum :default "NewEnumerator0"))
  (return (Utilities|Select :Index Quality :NewEnumerator0 "(R=1.000000,G=1.000000,B=1.000000,A=1.000000)" :NewEnumerator1 "(R=0.117647,G=1.000000,B=0.000000,A=1.000000)" :NewEnumerator2 "(R=0.000000,G=0.439216,B=0.866667,A=1.000000)" :NewEnumerator3 "(R=0.639216,G=0.207843,B=0.933333,A=1.000000)")))

(fn GetPowerLevel
  (params (Quality :type EQuality%20Enum :default "NewEnumerator0") (Type :type EItemType%20Enum :default "NewEnumerator0"))
  (switch Utilities|FlowControl|Switch|SwitchonEItemType Type
    (:NewEnumerator0
      ;[1 1 1] Weapon
      (return (Utilities|Select :Index Quality :NewEnumerator0 10 :NewEnumerator1 20 :NewEnumerator2 35 :NewEnumerator3 50)))
    (:NewEnumerator1
      ;[1 1 1] Utility
      (return (Utilities|Select :Index Quality :NewEnumerator0 8 :NewEnumerator1 20 :NewEnumerator2 35 :NewEnumerator3 60)))
    (:NewEnumerator2
      ;[1 1 1] Base
      (return (Utilities|Select :Index Quality :NewEnumerator0 0 :NewEnumerator1 0 :NewEnumerator2 0 :NewEnumerator3 0)))
    (:NewEnumerator3
      ;[1 1 1] Head
      (return (Utilities|Select :Index Quality :NewEnumerator0 0 :NewEnumerator1 0 :NewEnumerator2 0 :NewEnumerator3 0)))
    (:NewEnumerator4
      ;[1 1 1] Ammo
      (return (Utilities|Select :Index Quality :NewEnumerator0 0 :NewEnumerator1 0 :NewEnumerator2 0 :NewEnumerator3 0)))))

(fn GetModifierAmounts
  (params (Quality :type EQuality%20Enum :default "NewEnumerator0"))
  (switch Utilities|FlowControl|Switch|SwitchonEQuality Quality
    (:NewEnumerator0
      (return 0 1))
    (:NewEnumerator1
      (return 1 2))
    (:NewEnumerator2
      (return 1 3))
    (:NewEnumerator3
      (return 2 4))))

(fn GetMinimalPowerCost
  (params (Quality :type EQuality%20Enum :default "NewEnumerator0"))
  (return (Utilities|Select :Index Quality :NewEnumerator0 0 :NewEnumerator1 2 :NewEnumerator2 5 :NewEnumerator3 8)))