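; BPL_TileHelper is a map tile helper Blueprint that picks a random direction from a set of available ones.
; RandomDirection takes the available directions as a bitmask and loops over every EDirection value, testing the bit at two to the power of its enum index.
; Matching directions are collected in an array, and a uniformly random entry is returned as an EDirection, with no guard for an empty mask.
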(fn RandomDirection
  (params (AviableDirections :type Integer))
  (bind _aviabledirection (LocalVariables|GetAviableDirection))
  (bind _enumvalue (|ForEachEDirection)
    (:LoopBody
      (if (Math|Conversions|ToBoolean(Integer) (Class|KismetMathLibrary|AndIntInt AviableDirections (Math|Float|Floor (Math|Float|Power 2.0 (Math|Conversions|ToFloat(Integer) (Math|Conversions|ToInteger(Byte) _enumvalue))))))
        (Utilities|Array|Add (LocalVariables|GetAviableDirection) _enumvalue)))
    (:then
      (return (Utilities|Enum|ByteToEnumEDirection (Utilities|Array|Get(acopy) _aviabledirection (Math|Random|RandomIntegerinRange 0 (Utilities|Array|LastIndex _aviabledirection))))))))