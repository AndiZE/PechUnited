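; BP_MapGen generates a grid map of BP_Tile actors with the start of a path.
; CreateMap clears old tiles, spawns a row-major grid and links each tile to its previously spawned X and Y neighbours.
; CreatePath adds a random tile, sets a separately randomized tile's mesh to Spawn, then appends a neighbour of the last map tile.
; Its WayLenght countdown queries neighbours without extending the path, so path generation appears unfinished.
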(fn ConstructionScript)

(fn CreateMap
  (Utilities|FlowControl|Sequence
    (:then_0
      (CallFunction|ClearMap)
      (for _index (range 0 (- (Variables|Default|GetSizeY) 1))
        (for _index_2 (range 0 (- (Variables|Default|GetSizeX) 1))
          (bind _returnvalue (Game|SpawnActorfromClass "/Game/Blueprint/Map/BP_Tile.BP_Tile_C" (Math|Transform|MakeTransform (Math|Vector|MakeVector (* _index_2 (Variables|Default|GetTilesize)) (* _index (Variables|Default|GetTilesize)) 0.0) "0, 0, 0" "1,1,1") "AlwaysSpawn" 0 0))
          (Utilities|FlowControl|Sequence
            (:then_0
              (if (> _index_2 0)
                (Default|SetNeighbour _returnvalue "NewEnumerator2" (CallFunction|GetTile (- _index_2 1) _index))))
            (:then_1
              (if (> _index 0)
                (Default|SetNeighbour _returnvalue "NewEnumerator3" (CallFunction|GetTile _index_2 (- _index 1)))))
            (:then_2
              (Utilities|Array|Add (Variables|Default|GetMapTiles) _returnvalue))))))
    (:then_1
      (CallFunction|CreatePath))))

(fn ClearMap
  (for _array_element (Variables|Default|GetMapTiles)
    (Actor|DestroyActor _array_element))
  (Utilities|Array|Clear (Variables|Default|GetMapTiles)))

(fn CreatePath
  (bind _maptiles (Variables|Default|GetMapTiles))
  (bind _maptiles_2 (Variables|Default|GetMapTiles))
  (bind _path (LocalVariables|GetPath))
  (bind _returnvalue (Utilities|Array|LastIndex _maptiles))
  (bind _returnvalue_2 (Math|Random|RandomIntegerinRange 0 _returnvalue))
  (bind _output (Utilities|Array|Get(acopy) _maptiles _returnvalue_2))
  (Utilities|Array|Add (LocalVariables|GetPath) _output)
  (Components|StaticMesh|SetStaticMesh (Variables|/Game/Blueprint/Map/BP_Tile.BP_Tile_C|GetMesh _output) "/Game/Models/Path/Spawn.Spawn")
  (bind _neighbour (Default|GetNeighbour (Utilities|Array|Get(acopy) _maptiles_2 (Utilities|Array|LastIndex _maptiles_2)) "NewEnumerator0"))
  (Utilities|Array|Add (LocalVariables|GetPath) _neighbour)
  (Math|Integer|DecrementInt (LocalVariables|GetWayLenght)
    (:%20%20
      (while (> (LocalVariables|GetWayLenght) 0)
        (Math|Integer|DecrementInt (LocalVariables|GetWayLenght)
          (:%20%20
            (Default|GetNeighbour (Utilities|Array|Get(acopy) _path (Utilities|Array|LastIndex _path)) "NewEnumerator0")))))))

(fn GetTile
  (params (XPos :type Integer) (YPos :type Integer))
  (return (Utilities|Array|Get(acopy) (Variables|Default|GetMapTiles) (+ XPos (* YPos (Variables|Default|GetSizeX))))))