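; BP_Tile is a map tile that forms one piece of a path running from spawn to goal.
; It links neighbours both ways by direction and reports inactive ones, excluding the incoming side, as available connections.
; Connections are stored as four-direction bitmasks, which UpdateMesh maps to a spawn, goal, straight or corner mesh and its yaw.
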(fn ConstructionScript)

(fn SetNeighbour
  (params (Direction :type EDirection%20Enum :default "NewEnumerator0") (Neighbour :type BP%20Tile%20Object%20Reference))
  (Utilities|Array|SetArrayElem (Variables|Default|GetNeighbours) (Math|Conversions|ToInteger(Byte) Direction) Neighbour)
  (Utilities|Array|SetArrayElem (Variables|BP_Tile_C|GetNeighbours Neighbour) (Math|Conversions|ToInteger(Byte) (Utilities|GetOpposite Direction)) self))

(fn GetNeighbour
  (params (Direction :type EDirection%20Enum :default "NewEnumerator0"))
  (bind _returnvalue (Math|Conversions|ToInteger(Byte) Direction))
  (bind _neighbours (Variables|Default|GetNeighbours))
  (bind _output (Utilities|Array|Get(acopy) _neighbours _returnvalue))
  (Utilities|IsValid _output
    (:Is%20Valid
      (return _output))
    (:Is%20Not%20Valid
      (return 0))))

(fn GetAviableConnection
  (params (FromDirection :type EDirection%20Enum :default "NewEnumerator0"))
  (for (_array_element _array_index) (Variables|Default|GetNeighbours)
    (Utilities|IsValid _array_element
      (:Is%20Valid
        (if (and (not (Variables|BP_Tile_C|GetPathActive _array_element)) (!= _array_index (Math|Conversions|ToInteger(Byte) FromDirection)))
          (Variables|Default|SetAviablePaths (Class|KismetMathLibrary|OrIntInt (Math|Float|Floor (Math|Float|Power 2.0 (Math|Conversions|ToFloat(Integer) _array_index))) (Variables|Default|GetAviablePaths)))))))
  (return (Variables|Default|GetAviablePaths)))

(fn UpdateMesh
  (params (StartTile :type Boolean) (EndTile :type Boolean))
  (bind _returnvalue (|BitmaskLiteral 9))
  (bind _returnvalue_2 (|BitmaskLiteral 12))
  (bind _returnvalue_3 (|BitmaskLiteral 5))
  (bind _returnvalue_4 (|BitmaskLiteral 10))
  (bind _returnvalue_5 (|BitmaskLiteral 3))
  (bind _returnvalue_6 (|BitmaskLiteral 6))
  (bind _connectedpaths (Variables|Default|GetConnectedPaths))
  (bind _connectedpaths_2 (Variables|Default|GetConnectedPaths))
  (bind _connectedpaths_3 (Variables|Default|GetConnectedPaths))
  (bind _connectedpaths_4 (Variables|Default|GetConnectedPaths))
  (bind _connectedpaths_5 (Variables|Default|GetConnectedPaths))
  (bind _connectedpaths_6 (Variables|Default|GetConnectedPaths))
  (bind _returnvalue_7 (== _connectedpaths_6 _returnvalue))
  (bind _returnvalue_8 (== _connectedpaths _returnvalue_3))
  (bind _returnvalue_9 (== _connectedpaths_2 _returnvalue_4))
  (bind _returnvalue_10 (== _connectedpaths_3 _returnvalue_5))
  (bind _returnvalue_11 (== _connectedpaths_4 _returnvalue_6))
  (bind _returnvalue_12 (== _connectedpaths_5 _returnvalue_2))
  (Utilities|FlowControl|Sequence
    (:then_0
      (if (or StartTile EndTile)
        (if StartTile
          (Components|StaticMesh|SetStaticMesh (Variables|Default|GetMesh) "/Game/Models/Path/Spawn.Spawn")
          (else
            (Components|StaticMesh|SetStaticMesh (Variables|Default|GetMesh) "/Game/Models/Path/Goal.Goal")))
        (bind _enumvalue (|ForEachEDirection)
          (:LoopBody
            (if (== (Math|Float|Floor (Math|Float|Power 2.0 (Math|Conversions|ToFloat(Integer) (Math|Conversions|ToInteger(Byte) _enumvalue)))) (Variables|Default|GetConnectedPaths))
              (LocalVariables|SetRotation (* (Math|Conversions|ToFloat(Integer) (Math|Conversions|ToInteger(Byte) _enumvalue)) 9e+01)))))
        (elif (or _returnvalue_8 _returnvalue_9)
          (Components|StaticMesh|SetStaticMesh (Variables|Default|GetMesh) "/Game/Models/Path/Straight.Straight")
          (Utilities|FlowControl|Sequence
            (:then_0
              (if _returnvalue_8
                (LocalVariables|SetRotation 0.0)))
            (:then_1
              (if _returnvalue_9
                (LocalVariables|SetRotation 9e+01))))
          (elif (Math|Boolean|ORBoolean _returnvalue_10 _returnvalue_11 _returnvalue_12 _returnvalue_7)
            (Components|StaticMesh|SetStaticMesh (Variables|Default|GetMesh) "/Game/Models/Path/Corner.Corner")
            (Utilities|FlowControl|Sequence
              (:then_0
                (if _returnvalue_10
                  (LocalVariables|SetRotation 0.0)))
              (:then_1
                (if _returnvalue_11
                  (LocalVariables|SetRotation 9e+01)))
              (:then_2
                (if _returnvalue_12
                  (LocalVariables|SetRotation 1.8e+02)))
              (:then_3
                (if _returnvalue_7
                  (LocalVariables|SetRotation 2.7e+02))))))))
    (:then_1
      (Transformation|SetWorldRotation (Variables|Default|GetMesh) (Math|Rotator|MakeRotator 0.0 0.0 (LocalVariables|GetRotation)) false false))))

(fn SetActiveConnection
  (params (Direction :type EDirection%20Enum :default "NewEnumerator0"))
  (Variables|Default|SetConnectedPaths (Class|KismetMathLibrary|OrIntInt (Math|Float|Floor (Math|Float|Power 2.0 (Math|Conversions|ToFloat(Integer) (Math|Conversions|ToInteger(Byte) Direction)))) (Variables|Default|GetConnectedPaths))))